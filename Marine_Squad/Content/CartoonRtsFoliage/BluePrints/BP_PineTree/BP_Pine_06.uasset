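; BP_Pine_06 is a clickable pine tree foliage actor that shakes on cursor hover and dissolves away when clicked.
; A click plays a one-shot animation while a timeline drives the Dissolve material parameter, then destroys the actor.
; The construction script optionally box-traces to snap and align the tree to the Landscape, and randomizes hue, scale and rotation through two toggle booleans.
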(event `self.ReceiveActorOnClicked`
  (params (ButtonPressed :type "Key Structure" :default "AnyKey"))
  ;[1 1 1] Create a dissolve dynamic material and a on click animation
  (`/Engine/EditorBlueprintResources/StandardMacros.DoOnce` false
    (:`Completed`
      (bind _output_get (set `self.bAutoDestroyWhenFinished` true))
      (bind _returnvalue (`PrimitiveComponent.CreateDynamicMaterialInstance` (`self.SkeletalMeshComponent`) 0 (`PrimitiveComponent.GetMaterial` (`self.SkeletalMeshComponent`) 0)))
      (set `self.DissolveMaterial` _returnvalue)
      (`SkeletalMeshComponent.PlayAnimation` (`self.SkeletalMeshComponent`) "/Game/CartoonRtsFoliage/Meshes/Trees/PineTree/Tree_Animation_01.Tree_Animation_01" false)
      ;[1 1 1] Destroy actor on finish
      (bind (_direction _newtrack_0) (`Timeline|Timeline_0`)
        (:`Update`
          (`MaterialInstanceDynamic.SetScalarParameterValue` (`self.DissolveMaterial`) "Dissolve" _newtrack_0))
        (:`Finished`
          (`self.K2_DestroyActor`))))))

(event `self.ReceiveActorBeginCursorOver`
  ;[1 1 1] Loop The oncursorOver Animation
  (if (not (stale `self.ReceiveActorOnClicked` _output_get))
    (`/Engine/EditorBlueprintResources/StandardMacros.DoOnce` false :!label _label
      (:`Completed`
        (`SkeletalMeshComponent.PlayAnimation` (`self.SkeletalMeshComponent`) "/Game/CartoonRtsFoliage/Meshes/Trees/PineTree/ShakeAnim.ShakeAnim" false)
        (goto _label :!via `Reset`)))))

(event `self.ReceiveBeginPlay`)

(fn `Parent_Transforms`
  (bind _returnvalue (`KismetMathLibrary.RandomFloatInRange` 0.0 10.0))
  (bind _returnvalue_2 (`KismetMathLibrary.RandomFloatInRange` (`self.SizeMin`) (`self.SizeMax`)))
  ;[1 1 1] Create Dynamic Material Instance
  (bind _returnvalue_3 (`PrimitiveComponent.CreateDynamicMaterialInstance` (`self.SkeletalMeshComponent`) 0 (`PrimitiveComponent.GetMaterial` (`self.SkeletalMeshComponent`) 0)))
  (set `self.Hue Material` _returnvalue_3)
  ;[1 1 1] Random Size, Hue and Rotation
  (`MaterialInstanceDynamic.SetScalarParameterValue` (`self.Hue Material`) "Hue" (`KismetMathLibrary.RandomFloatInRange` 0.0 1.0))
  (`SceneComponent.SetWorldScale3D` (`self.SkeletalMeshComponent`) (`KismetMathLibrary.MakeVector` _returnvalue_2 _returnvalue_2 _returnvalue_2))
  (`SceneComponent.K2_SetWorldRotation` (`self.SkeletalMeshComponent`) (`KismetMathLibrary.MakeRotator` _returnvalue _returnvalue (`KismetMathLibrary.RandomFloatInRange` 0.0 360.0)) false false))

(fn `UpdatePosition`
  (bind _returnvalue (`self.K2_GetActorLocation`))
  ;[1 1 1] Check with a boxTrace The actor location with the landscape
  (bind _outhit (`KismetSystemLibrary.BoxTraceSingle` (+ _returnvalue (0.0 0.0 5000.0)) (- _returnvalue (0.0 0.0 5000.0)) (25.0 25.0 10.0) (struct) "TraceTypeQuery3"))
  (bind (_bblockinghit _binitialoverlap _time _location _impactpoint _normal _impactnormal _physmat _hitactor) (`GameplayStatics.BreakHitResult` _outhit))
  ;[1 1 1] Align the mesh with the landscape
  (if (== (`GameplayStatics.GetObjectClass` _hitactor) "/Script/Landscape.Landscape")
    (`self.K2_SetActorLocation` (+ _location (`self.TreeOfset`)))
    (`self.K2_SetActorRotation` (`KismetMathLibrary.MakeRotFromZ` _normal))))

(fn `UserConstructionScript`
  ;[1 1 1] Set Booleans to easily trigger the construction script or disable the update pos with the landscape
  (if (`self.UpdatePos`)
    (`self.UpdatePosition`))
  (if (`self.ActivateConstructionScript`)
    (`self.Parent_Transforms`)))