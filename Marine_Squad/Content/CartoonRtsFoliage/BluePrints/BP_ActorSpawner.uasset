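; Foliage spawner volume that scatters random actors from ActorList over the landscape or a target mesh, attached to itself.
; SpawnTrees runs SpawnTree in batches while the requested total is below a cap; Deleteobject destroys spawned actors.
; Random box traces through the bounds (top-down for landscape, multi-axis for meshes) place actors along hit normals, optionally filtered by physical material.
; UpdatesActors toggles BP_Pine_06 booleans to retrigger their construction scripts.
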(event `UpdatesActors`
  ;[1 1 1] Modify actors booleans to trigger the construciton script  (cast to another blueprint)
  (for _array_element (`self.Spawned actor`)
    (bind _asbp_pine_06 (cast `/Game/CartoonRtsFoliage/BluePrints/BP_PineTree/BP_Pine_06` _array_element))
    (`|ExecutionSequence`
      (:`then_0`
        (if (`/Game/CartoonRtsFoliage/BluePrints/BP_PineTree/BP_Pine_06.ActivateConstructionScript` _asbp_pine_06)
          (set `/Game/CartoonRtsFoliage/BluePrints/BP_PineTree/BP_Pine_06.ActivateConstructionScript` false _asbp_pine_06)
          (else
            (set `/Game/CartoonRtsFoliage/BluePrints/BP_PineTree/BP_Pine_06.ActivateConstructionScript` true _asbp_pine_06))))
      (:`then_1`
        (if (`/Game/CartoonRtsFoliage/BluePrints/BP_PineTree/BP_Pine_06.UpdatePos` _asbp_pine_06)
          (set `/Game/CartoonRtsFoliage/BluePrints/BP_PineTree/BP_Pine_06.UpdatePos` false _asbp_pine_06)
          (else
            (set `/Game/CartoonRtsFoliage/BluePrints/BP_PineTree/BP_Pine_06.UpdatePos` true _asbp_pine_06)))))))

(event `Delete object`
  ;[1 1 1] Delete Actors in the array
  (set `self.Total Number Spawned` 0)
  (`self.K2_DestroyActor` (`self.Spawned actor`)))

(event `SpawnTrees`
  ;[1 1 1] Spawn the Actors
  (if (< (`self.Total Number Spawned`) (`self.Max Number Spawned`))
    (`self.SpawnTree` (`self.Spawn Number`) (`self.ActorList`))
    (set `self.Total Number Spawned` (+ (`self.Spawn Number`) (`self.Total Number Spawned`)))))

(fn `SpawnTree`
  (params (SpawnNumber :type Integer :default 5) (ActorList :type "Array of Actor Class Reference"))
  (bind (_origin _boxextent) (`self.GetActorBounds` false))
  (bind (_origin_2 _boxextent_2) (`self.GetActorBounds` false))
  (bind (_origin_3 _boxextent_3) (`self.GetActorBounds` false))
  (bind (_origin_4 _boxextent_4) (`self.GetActorBounds` false))
  (bind (_origin_5 _boxextent_5) (`self.GetActorBounds` false))
  (bind (_origin_6 _boxextent_6) (`self.GetActorBounds` false))
  (bind _actorlist (`self.ActorList`))
  (bind _actorlist_2 (`self.ActorList`))
  (bind _x (.x _boxextent))
  (bind _z (.z _boxextent))
  (bind _y (.y _boxextent_2))
  (bind _z_2 (.z _boxextent_2))
  (bind _x_2 (.x _boxextent_3))
  (bind _y_2 (.y _boxextent_3))
  (bind _x_3 (.x _boxextent_4))
  (bind _z_3 (.z _boxextent_4))
  (bind _x_4 (.x _boxextent_5))
  (bind _y_3 (.y _boxextent_5))
  (bind _y_4 (.y _boxextent_6))
  (bind _z_4 (.z _boxextent_6))
  (bind _returnvalue (+ _origin_6 (`KismetMathLibrary.MakeVector` (.x _origin_6) (`KismetMathLibrary.RandomFloatInRange` (- _y_4 (* _y_4 2.0)) _y_4) (`KismetMathLibrary.RandomFloatInRange` (- _z_4 (* _z_4 2.0)) _z_4))))
  (bind _returnvalue_2 (+ _origin (`KismetMathLibrary.MakeVector` (`KismetMathLibrary.RandomFloatInRange` (- _x (* _x 2.0)) _x) (.y _origin) (`KismetMathLibrary.RandomFloatInRange` (- _z (* _z 2.0)) _z))))
  (bind _returnvalue_3 (+ _origin_4 (`KismetMathLibrary.MakeVector` (`KismetMathLibrary.RandomFloatInRange` (- _x_3 (* _x_3 2.0)) _x_3) (.y _origin_4) (`KismetMathLibrary.RandomFloatInRange` (- _z_3 (* _z_3 2.0)) _z_3))))
  (bind _returnvalue_4 (+ _origin_2 (`KismetMathLibrary.MakeVector` (.x _origin_2) (`KismetMathLibrary.RandomFloatInRange` (- _y (* _y 2.0)) _y) (`KismetMathLibrary.RandomFloatInRange` (- _z_2 (* _z_2 2.0)) _z_2))))
  (bind _returnvalue_5 (+ _origin_3 (`KismetMathLibrary.MakeVector` (`KismetMathLibrary.RandomFloatInRange` (- _x_2 (* _x_2 2.0)) _x_2) (`KismetMathLibrary.RandomFloatInRange` (- _y_2 (* _y_2 2.0)) _y_2) (.z _origin_3))))
  (bind _returnvalue_6 (+ _origin_5 (`KismetMathLibrary.MakeVector` (`KismetMathLibrary.RandomFloatInRange` (- _x_4 (* _x_4 2.0)) _x_4) (`KismetMathLibrary.RandomFloatInRange` (- _y_3 (* _y_3 2.0)) _y_3) (.z _origin_5))))
  (bind _returnvalue_7 (- _returnvalue_5 (0.0 0.0 5000.0)))
  (bind _returnvalue_8 (+ _returnvalue_5 (0.0 0.0 5000.0)))
  ;[1 1 1] Set variable for number of loop to proceed
  (set `self.Spawn Number` SpawnNumber)
  (set `self.ActorList` ActorList)
  (for _ (range 1 (+ (`self.Spawn Number`) 1))
    (if (`self.SpawnToLandscape`)
      ;[1 1 1] Box Trace with the landscape and spawn on the corresponding physics material
      (bind _outhit (`KismetSystemLibrary.BoxTraceSingle` _returnvalue_8 _returnvalue_7 (10.0 10.0 5.0) (struct) (`self.Landscape`) true))
      (if (`self.SpawnToLandscape`)
        (bind (_bblockinghit _binitialoverlap _time _location _impactpoint _normal _impactnormal _physmat _hitactor) (`GameplayStatics.BreakHitResult` _outhit))
        (if (== (`GameplayStatics.GetObjectClass` _hitactor) (`self.objectClass`))
          (if (`self.SpawnEveryWhere`)
            (bind _returnvalue_9 (`|SpawnActorFromClass` (`KismetArrayLibrary.Array_Get` _actorlist_2 (`KismetMathLibrary.RandomInteger` (`KismetArrayLibrary.Array_Length` _actorlist_2))) (`KismetMathLibrary.MakeTransform` (+ _location (`self.TreeOfset`)) (`KismetMathLibrary.MakeRotFromZ` _normal)) "AlwaysSpawn" "OverrideRootScale" :!label _label))
            ;[1 1 1] Add spawned actor in an array and attach them to the spawner volume.
            (`KismetArrayLibrary.Array_Add` (`self.Spawned actor`) _returnvalue_9)
            (`self.K2_AttachToActor` _returnvalue_9 self "None" "KeepWorld" "KeepWorld" "KeepWorld" true)
            (elif (== _physmat (`self.SpawnerArea`))
              (goto _label)))))
      (else
        (for _array_element (`|MakeArray` _returnvalue_8 (+ _returnvalue_4 (5000.0 0.0 0.0)) (+ _returnvalue_2 (0.0 5000.0 0.0)) (+ _returnvalue_3 (0.0 -5000.0 0.0)) (+ _returnvalue (-5000.0 0.0 0.0)) (+ _returnvalue_6 (0.0 0.0 -5000.0)))
          (for _array_element_2 (`|MakeArray` _returnvalue_7 (- _returnvalue_4 (5000.0 0.0 0.0)) (- _returnvalue_2 (0.0 5000.0 0.0)) (- _returnvalue (-5000.0 0.0 0.0)) (- _returnvalue_3 (0.0 -5000.0 0.0)) (- _returnvalue_6 (0.0 0.0 -5000.0)))
            ;[1 1 1] Box Trace with the landscape and spawn on the corresponding physics material
            (bind _outhit_2 (`KismetSystemLibrary.BoxTraceSingle` _array_element_2 _array_element (10.0 10.0 5.0) (struct) (`self.Landscape`) true))
            (if (`self.SpawnToLandscape`)
              (bind (_bblockinghit_2 _binitialoverlap_2 _time_2 _location_2 _impactpoint_2 _normal_2 _impactnormal_2 _physmat_2 _hitactor_2) (`GameplayStatics.BreakHitResult` _outhit_2))
              (if (== (`GameplayStatics.GetObjectClass` _hitactor_2) (`self.objectClass`))
                (if (`self.SpawnEveryWhere`) :!label _label_2
                  (bind _returnvalue_10 (`|SpawnActorFromClass` (`KismetArrayLibrary.Array_Get` _actorlist (`KismetMathLibrary.RandomInteger` (`KismetArrayLibrary.Array_Length` _actorlist))) (`KismetMathLibrary.MakeTransform` (+ _location_2 (`self.TreeOfset`)) (`KismetMathLibrary.MakeRotFromZ` _normal_2)) "AlwaysSpawn" "OverrideRootScale" :!label _label_3))
                  ;[1 1 1] Add spawned actor in an array and attach them to the spawner volume.
                  (`KismetArrayLibrary.Array_Add` (`self.Spawned actor`) _returnvalue_10)
                  (`self.K2_AttachToActor` _returnvalue_10 self "None" "KeepWorld" "KeepWorld" "KeepWorld" true)
                  (elif (== _physmat_2 (`self.SpawnerArea`))
                    (goto _label_3))))
              (elif (== _hitactor_2 (`self.MeshToSpawn`))
                (goto _label_2)))))))))

(fn `UserConstructionScript`)