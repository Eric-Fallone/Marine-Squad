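; Base gameplay ability that lets the player pick a target unit, then fires a fireball and applies ground-blast damage.
; It flags the player controller as confirming while a user-confirmed WaitTargetData task runs with the BP_BaseAbilityChooseUnit target actor.
; Valid data commits the ability, spawns FireBall_Projectile with that unit as target and applies GE_GroundBlast_Damage immediately, not on impact.
; Both outcomes clear the flag, but only cancellation calls EndAbility.
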(event `self.K2_ActivateAbility`
  (bind _asmy_player_controller_marine_squ_bp (cast `/Game/BP/MyPlayerController_MarineSqu_BP` (`GameplayStatics.GetPlayerController` 0)))
  (set `PlayerController_MarineSquad.isAbilityBeingConfirmed` true _asmy_player_controller_marine_squ_bp)
  (bind (_asynctaskproxy _data) (`AbilityTask_WaitTargetData.WaitTargetData` "None" "UserConfirmed" "/Game/BP/Units_BP/Abilities/ChooseUnit/BP_BaseAbilityChooseUnit.BP_BaseAbilityChooseUnit_C" 0.0 (struct) (struct) null)
    (:`ValidData`
      (set `PlayerController_MarineSquad.isAbilityBeingConfirmed` false _asmy_player_controller_marine_squ_bp)
      (`self.K2_CommitAbility`)
      (bind _asparent_unit (cast `ParentUnit` (`|GetArrayItem` (`AbilitySystemBlueprintLibrary.GetActorsFromTargetData` _data))))
      (bind (_asynctaskproxy_2 _spawnedactor) (`AbilityTask_SpawnActor.SpawnActor` (struct) "/Game/BP/Units_BP/Projectiles/FireBall_Projectile.FireBall_Projectile_C" _asparent_unit null)
        (:`then`
          (`self.BP_ApplyGameplayEffectToTarget` _data "/Game/BP/Units_BP/Abilities/AOE_choose_location/GE_GroundBlast_Damage.GE_GroundBlast_Damage_C"))
        (:`Success`
          (cast `/Game/BP/Units_BP/Projectiles/FireBall_Projectile` _spawnedactor))))
    (:`Cancelled`
      (set `PlayerController_MarineSquad.isAbilityBeingConfirmed` false _asmy_player_controller_marine_squ_bp)
      (`self.K2_EndAbility`))))