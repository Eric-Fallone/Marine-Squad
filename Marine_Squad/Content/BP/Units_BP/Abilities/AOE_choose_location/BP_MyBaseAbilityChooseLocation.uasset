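; Base ability actor for choosing a target location, such as for an area-of-effect cast, within Range of the casting unit.
; BeginPlay caches the MarineSqu player controller, whose HUD supplies the mouse world position each Tick.
; TargetLocation follows the mouse within range, otherwise it is clamped to the range edge along the direction from the unit's capsule to the mouse.
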(event `self.ReceiveBeginPlay`
  (bind _asmy_player_controller_marine_squ_bp (cast `/Game/BP/MyPlayerController_MarineSqu_BP` (`GameplayStatics.GetPlayerController` 0))))

(event `self.ReceiveTick`
  (params (DeltaSeconds :type "Float (single-precision)"))
  (bind _range (`self.Range`))
  (bind _returnvalue (`SceneComponent.K2_GetComponentLocation` (`Character.CapsuleComponent` (`self.CastingUnit`))))
  (bind _returnvalue_2 (`HUD_MarineSquad.GetMouseWorldPos` (`PlayerController_MarineSquad.HUDPtr` (stale `self.ReceiveBeginPlay` _asmy_player_controller_marine_squ_bp))))
  (`/Engine/EditorBlueprintResources/StandardMacros.CompareFloat` (`KismetMathLibrary.Vector_Distance` _returnvalue_2 _returnvalue) _range
    (:`>`
      (set `self.TargetLocation` (+ (* (`KismetMathLibrary.Normal` (- _returnvalue_2 _returnvalue)) _range) _returnvalue)) ; snaps to edge of range
    )
    (:`==`
      (set `self.TargetLocation` _returnvalue_2 :!label _label) ; mouse is within range of the target
    )
    (:`<`
      (goto _label))))

(fn `UserConstructionScript`)